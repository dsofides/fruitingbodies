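; Player camera controller for a mouse-driven orbit view, with rotation and zoom on a spring arm and a Canvas widget created at BeginPlay.
; Turn and LookUp axes rotate the arm while CanRotate is set, by the Camera Rotate action or a left press that hits nothing under the cursor.
; Mouse wheel steps a target arm length between near and far limits, which Tick smoothly lerps toward.
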(event EventBeginPlay
  (bind _returnvalue (Game|GetPlayerController 0))
  (Utilities|FlowControl|Sequence
    (:then_0
      (Input|SetInputModeGameandUI _returnvalue 0 "LockAlways" false)
      (Variables|/Script/Engine.PlayerController|SetbShowMouseCursor _returnvalue true)
      (bind _returnvalue_2 (UserInterface|CreateWidget "/Game/UI/Canvas.Canvas_C" _returnvalue))
      (bind _output_get (Variables|Default|SetCanvas _returnvalue_2))
      (UserInterface|Viewport|AddtoViewport _output_get 0)
      (Variables|Default|SetArm%20Target%20Length (Variables|/Script/Engine.SpringArmComponent|GetTargetArmLength (Variables|Default|GetSpringArm))))))

(event EventTick
  (params (DeltaSeconds :type Float%20%28single-precision%29))
  (bind _springarm (Variables|Default|GetSpringArm))
  (Variables|/Script/Engine.SpringArmComponent|SetTargetArmLength _springarm (Math|Float|Lerp (Variables|/Script/Engine.SpringArmComponent|GetTargetArmLength _springarm) (Variables|Default|GetArm%20Target%20Length) (* DeltaSeconds 5.0))))

(event Input|ActionEvents|InputActionCameraRotate
  (params (Key :type Key%20Structure :default "None"))
  (:Pressed
    (Variables|Default|SetCan%20Rotate true))
  (:Released
    (Variables|Default|SetCan%20Rotate false)))

(event Input|AxisEvents|InputAxisLookUp
  (params (AxisValue :type Float%20%28single-precision%29))
  (if (Variables|Default|GetCan%20Rotate)
    (Transformation|SetWorldRotation (Variables|Default|GetSpringArm) (Math|Rotator|CombineRotators (Math|Rotator|MakeRotator 0.0 AxisValue 0.0) (Transformation|GetWorldRotation (Variables|Default|GetSpringArm))) false false)))

(event Input|AxisEvents|InputAxisTurn
  (params (AxisValue :type Float%20%28single-precision%29))
  (if (Variables|Default|GetCan%20Rotate)
    (Transformation|SetWorldRotation (Variables|Default|GetSpringArm) (Math|Rotator|CombineRotators (Transformation|GetWorldRotation (Variables|Default|GetSpringArm)) (Math|Rotator|MakeRotator 0.0 0.0 AxisValue)) false false)))

(event Input|MouseEvents|MouseWheelUp
  (params (Key :type Key%20Structure :default "None"))
  (:Pressed
    (if (> (Variables|Default|GetArm%20Target%20Length) (Variables|Default|GetCamera%20Zoom%20Near%20Limit))
      (Variables|Default|SetArm%20Target%20Length (+ (Variables|Default|GetArm%20Target%20Length) (* (Variables|Default|GetZoom%20Scale) -1.0))))))

(event Input|MouseEvents|MouseWheelDown
  (params (Key :type Key%20Structure :default "None"))
  (:Pressed
    (if (< (Variables|Default|GetArm%20Target%20Length) (Variables|Default|GetCamera%20Zoom%20Far%20Limit))
      (Variables|Default|SetArm%20Target%20Length (+ (Variables|Default|GetArm%20Target%20Length) (Variables|Default|GetZoom%20Scale))))))

(event Input|MouseEvents|LeftMouseButton
  (params (Key :type Key%20Structure :default "None"))
  (:Pressed
    (if (.bBlockingHit (Collision|BreakHitResult (.HitResult (Game|Player|GetHitResultUnderCursorbyChannel (Game|GetPlayerController 0) "TraceTypeQuery1" true))))
      (Variables|Default|SetCan%20Rotate false)
      (else
        (Variables|Default|SetCan%20Rotate true))))
  (:Released
    (Variables|Default|SetCan%20Rotate false)))

(fn ConstructionScript)